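; Actor that shows the shared community cards (flop, turn and river) on a poker table.
; On BeginPlay it caches five BP_CardVisualizer child actors into an ordered array.
; Update events set each visualizer face-up with the incoming card data by index and unhide it; the hide event hides them all.
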(event `self.ReceiveBeginPlay`
  (`self.InitializeCardRef`))

(event `CommunityCardDisplayInterface.UpdateCommunityCards`
  (params (CommunityCards :type "Array of Card Structure (by ref)"))
  (`self.Display Community Cards` CommunityCards))

(event `CommunityCardDisplayInterface.HideCommunityCards`
  (`self.ClearCommunityCards`))

(fn `ClearCommunityCards`
  (for _array_element (`self.LocalVisualizersArray`)
    (`/Engine/EditorBlueprintResources/StandardMacros.IsValid` _array_element
      (:`Is Valid`
        (`self.SetActorHiddenInGame` _array_element true)
        (`KismetSystemLibrary.PrintString` "Clear CommunityCards")))))

(fn `Display Community Cards`
  (params (ArrayCard :type "Array of Card Structure"))
  (for (_array_element _array_index) ArrayCard
    (bind _output (`|GetArrayItem` (`self.LocalVisualizersArray`) _array_index))
    (`/Engine/EditorBlueprintResources/StandardMacros.IsValid` _output
      (:`Is Valid`
        (`/Game/Blueprints/Actors/BP_CardVisualizer.Initialize Card and Set Visuals` _output true _array_element)
        (`self.SetActorHiddenInGame` _output false)
        (`KismetSystemLibrary.PrintString` "DisplayCommunityCards")))))

(fn `InitializeCardRef`
  (`|ExecutionSequence`
    (:`then_0`
      (bind _asbp_card_visualizer (cast `/Game/Blueprints/Actors/BP_CardVisualizer` (`ChildActorComponent.ChildActor` (`self.CardVisualizer_Flop1_CAC`))))
      (set `self.FlopCard1_Vis` _asbp_card_visualizer))
    (:`then_1`
      (bind _asbp_card_visualizer_2 (cast `/Game/Blueprints/Actors/BP_CardVisualizer` (`ChildActorComponent.ChildActor` (`self.CardVisualizer_Flop2_CAC`))))
      (set `self.FlopCard2_Vis` _asbp_card_visualizer_2))
    (:`then_2`
      (bind _asbp_card_visualizer_3 (cast `/Game/Blueprints/Actors/BP_CardVisualizer` (`ChildActorComponent.ChildActor` (`self.CardVisualizer_Flop3_CAC`))))
      (set `self.FlopCard3_Vis` _asbp_card_visualizer_3))
    (:`then_3`
      (bind _asbp_card_visualizer_4 (cast `/Game/Blueprints/Actors/BP_CardVisualizer` (`ChildActorComponent.ChildActor` (`self.CardVisualizer_Turn_CAC`))))
      (set `self.TurnCard_Vis` _asbp_card_visualizer_4))
    (:`then_4`
      (bind _asbp_card_visualizer_5 (cast `/Game/Blueprints/Actors/BP_CardVisualizer` (`ChildActorComponent.ChildActor` (`self.CardVisualizer_River_CAC`))))
      (set `self.RiverCard_Vis` _asbp_card_visualizer_5))
    (:`then_5`
      (set `self.LocalVisualizersArray` (`|MakeArray` (`self.FlopCard1_Vis`) (`self.FlopCard2_Vis`) (`self.FlopCard3_Vis`) (`self.TurnCard_Vis`) (`self.RiverCard_Vis`))))))

(fn `UserConstructionScript`)