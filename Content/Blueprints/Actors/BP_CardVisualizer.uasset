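; BP_CardVisualizer is an actor that displays a playing card face on a plane mesh, based on its CardData suit and rank.
; ShowCard creates a dynamic instance of MI_Card_Dynamic on PlaneMesh and builds a Suit_Rank row name from the enum strings.
; That row in CardTextureDataTable supplies the face texture for the CardTexture parameter, and a missing row prints an error.
; The event graph and construction script are empty, so ShowCard runs only when called.
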(fn `ShowCard`
  (locals (LocalDMI :type "MaterialInstanceDynamic Object Reference"))
  (bind (_suit _rank) (break `Card` (`self.CardData`)))
  (bind _returnvalue (`KismetStringLibrary.Concat_StrStr` (`KismetStringLibrary.Concat_StrStr` (`|GetEnumeratorNameAsString` _suit) "_") (`|GetEnumeratorNameAsString` _rank)))
  (bind _returnvalue_2 (`PrimitiveComponent.CreateDynamicMaterialInstance` (`self.PlaneMesh`) 0 "/Game/Materials/MI_Card_Dynamic.MI_Card_Dynamic" "None"))
  (set `local.LocalDMI` _returnvalue_2)
  (bind _returnvalue_3 (`|GetDataTableRow` (`self.CardTextureDataTable`) (`KismetStringLibrary.Conv_StringToName` _returnvalue))
    (:`then`
      (`MaterialInstanceDynamic.SetTextureParameterValue` (`local.LocalDMI`) "CardTexture" (`.FaceTexture_8_38F30D374991C4C5E33A7CBF03002117` (break `/Game/Blueprints/GameLogicClasses/S_CardTextureData` _returnvalue_3))))
    (:`RowNotFound`
      (`KismetSystemLibrary.PrintString` (`KismetStringLibrary.Concat_StrStr` "Error: Card data not found in DataTable! Row Name^ " _returnvalue)))))

(fn `UserConstructionScript`)