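; Game mode for offline poker that sets up a match with one human player and bots, then starts the first hand.
; On BeginPlay it initializes the game instance's offline game manager from pending bot, stack and blind settings and plays level music, around short delays marked for removal.
; It sets seat visualizer visibility from occupied seat indices and teleports the player pawn to seat zero before dealing.
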(event `self.ReceiveBeginPlay`
  (bind _asmy_game_instance (cast `MyGameInstance` (`GameplayStatics.GetGameInstance`)))
  (`KismetSystemLibrary.Delay` 0.1) ; Убрать
  (bind _offlinegamemanager (`self.IntializeGameAndGameManager`))
  (`KismetSystemLibrary.Delay` 0.1) ; Убрать
  (bind _returnvalue (`GameplayStatics.SpawnSound2D` "/Game/Audio/Music/SC_GameMusic_Loop.SC_GameMusic_Loop" (`MyGameInstance.GameLevelMusicVolume` _asmy_game_instance) 1.0 0.0 null))
  (set `self.Sound_GameMusic` _returnvalue)
  (set `self.LocalSeats` (`OfflinePokerGameState.Seats` (`OfflineGameManager.GameStateData` _offlinegamemanager)))
  (bind _ispsvisualize (`self.InitializePlayerSeatVisualizers`))
  (if _ispsvisualize
    (`self.SpawnInRightPlace`)
    (`OfflineGameManager.StartNewHand` _offlinegamemanager)))

(fn `InitializePlayerSeatVisualizers`
  (returns (IsPSVisualize :type Boolean))
  (bind _outactors (`GameplayStatics.GetAllActorsOfClass` "/Game/Blueprints/Actors/BP_PlayerSeatVisualizer.BP_PlayerSeatVisualizer_C"))
  (for _array_element _outactors
    (bind _seatindexvizual (`/Game/Blueprints/Actors/BP_PlayerSeatVisualizer.SeatIndexVizual` _array_element))
    (message `PlayerSeatVisualizerInterface.SetSeatVisibility` _array_element (`KismetArrayLibrary.Array_IsValidIndex` (`self.LocalSeats`) _seatindexvizual))
    (if (== _seatindexvizual 0)
      (set `self.PlayerSeatVisualizer` _array_element)))
  (return true))

(fn `IntializeGameAndGameManager`
  (returns (OfflineGameManager :type "OfflineGameManager Object Reference"))
  (locals (DefaultNumBots :type Integer :default 3) (DefaultInitialStack :type Integer64 :default 300) (DefaultSmallBlind :type Integer64 :default 50))
  (bind _asmy_game_instance (cast `MyGameInstance` (`GameplayStatics.GetGameInstance`)))
  (bind _returnvalue (`MyGameInstance.GetOfflineGameManager` _asmy_game_instance))
  (`OfflineGameManager.InitializeGame` _returnvalue 1 (`MyGameInstance.PendingOfflineNumBots` _asmy_game_instance) (`MyGameInstance.PendingOfflineInitialStack` _asmy_game_instance) (`MyGameInstance.PendingSmallBlind` _asmy_game_instance))
  (return _returnvalue))

(fn `SpawnInRightPlace`
  (bind _playerseatvisualizer (`self.PlayerSeatVisualizer`))
  (bind _aspoker_player_controller (cast `PokerPlayerController` (`GameplayStatics.GetPlayerController` 0)))
  (bind _aspoker_player_pawn (cast `PokerPlayerPawn` (`Controller.K2_GetPawn` _aspoker_player_controller)))
  (`/Engine/EditorBlueprintResources/StandardMacros.IsValid` _playerseatvisualizer
    (:`Is Valid`
      (`self.K2_SetActorTransform` _aspoker_player_pawn (`self.GetTransform` _playerseatvisualizer) false true))
    (:`Is Not Valid`
      (`KismetSystemLibrary.PrintString` "InvalidPlayerSeatVisualizer"))))

(fn `UserConstructionScript`)